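; Top-down player character Blueprint with a zoomable spring-arm camera, movement modes and test montage playback.
; Aim, sprint and walk inputs set flags and call ChangeMovementState, while Space plays aim-dependent fire montages and V plays a death montage.
; The construction script configures the boom; the mouse wheel sets a clamped distance that Tick smoothly interpolates toward.
; CameraSlide is an empty stub, and camera shake is never triggered here.
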(event `Key|RightMouseButton`
  (params (Key :type "Key Structure"))
  (:`Pressed`
    (set `self.AimEnabled` true)
    (`self.ChangeMovementState` :!label _label))
  (:`Released`
    (set `self.AimEnabled` false)
    (goto _label)))

(event `InputAction|MovementModeChangeSprint`
  (params (Key :type "Key Structure"))
  (:`Pressed`
    (set `self.SprintRunEnabled` true)
    (goto _label))
  (:`Released`
    (set `self.SprintRunEnabled` false)
    (goto _label)))

(event `InputAction|AltChange`
  (params (Key :type "Key Structure"))
  (:`Pressed`
    (set `self.WalkEnabled` true)
    (goto _label))
  (:`Released`
    (set `self.WalkEnabled` false)
    (goto _label)))

(event `InputAxis|MouseWheel`
  (params (AxisValue :type "Float (single-precision)")))

(event `Key|F`
  (params (Key :type "Key Structure")))

(event `Key|RightMouseButton`
  (params (Key :type "Key Structure"))
  (:`Pressed`
    (`self.ChangeMovementState`))
  (:`Released`
    (`self.ChangeMovementState`)))

(event `self.ReceiveTick`
  (params (DeltaSeconds :type "Float (single-precision)"))
  (`self.Camera Zoom` DeltaSeconds))

(event `InputAxis|Zoom`
  (params (AxisValue :type "Float (single-precision)")))

(event `InputAxis|MouseWheel`
  (params (AxisValue :type "Float (single-precision)"))
  (set `self.Desired Camera Distance` (`KismetMathLibrary.FClamp` (+ (`self.Desired Camera Distance`) (* AxisValue -100.0)) 300.0 1200.0)))

(event `Key|SpaceBar`
  (params (Key :type "Key Structure"))
  (bind _mesh (`self.Mesh`))
  (:`Pressed`
    (if (`self.AimEnabled`)
      (`|PlayMontage` _mesh "/Game/Blueprint/Character/Mannequin/Animations/NewAnim/NewFire_Rifle_Hip_Montage.NewFire_Rifle_Hip_Montage")
      (else
        (`|PlayMontage` _mesh "/Game/Blueprint/Character/Mannequin/Animations/NewAnim/NewFire_Rifle_Ironsights_Montage.NewFire_Rifle_Ironsights_Montage")))))

(event `Key|V`
  (params (Key :type "Key Structure"))
  (:`Pressed`
    (`|PlayMontage` (`self.Mesh`) "/Game/Blueprint/Character/Mannequin/Animations/NewAnim/NewDeath_11_Montage.NewDeath_11_Montage")))

(fn `Camera Zoom`
  (params (DeltaTime1 :type "Float (double-precision)"))
  (locals (ZoomInput :type "Float (double-precision)") (DeltaTime :type "Float (double-precision)") (TargetArmLengthCurrent :type "Float (double-precision)" :default 600.0) (TargetArmLengthMin :type "Float (double-precision)" :default 150.0) (TargetArmLengthMax :type "Float (double-precision)" :default 1200.0) (ZoomSpeed :type "Float (double-precision)" :default 1000.0) (NewTargetArmLength :type "Float (double-precision)") (CurrentSpringArmLength :type "Float (double-precision)") (NewLocalVar_0 :type "Float (double-precision)" :default 0.0))
  (bind _cameraboom (`self.CameraBoom`))
  (set `SpringArmComponent.TargetArmLength` (`KismetMathLibrary.FInterpTo` (`SpringArmComponent.TargetArmLength` _cameraboom) (`self.Desired Camera Distance`) DeltaTime1 3.0) _cameraboom))

(fn `CameraShakeEvent`
  (`GameplayStatics.PlayWorldCameraShake` "/Game/Blueprint/Game/BP_ShakeCamera.BP_ShakeCamera_C" (`SceneComponent.K2_GetComponentLocation` (`self.TopDownCameraComponent`)) 0.0 30.0))

(fn `CameraSlide`
  (params (Value :type "Float (double-precision)"))
  (bind _hieghtcamerachangedistance (`self.HieghtCameraChangeDistance`))
  (if (!= Value 0.0)
    (if (< Value 0.0)
      (if (> (`self.HieghtCameraMax`) (+ 0.0 _hieghtcamerachangedistance))
        _)
      (elif (< (`self.HieghtCameraMin`) (- _hieghtcamerachangedistance 1.0))
        _))))

(fn `UserConstructionScript`
  (bind _cameraboom (`self.CameraBoom`))
  (set `SpringArmComponent.TargetArmLength` (`self.HieghtCameraMin`) _cameraboom)
  (`SceneComponent.K2_SetRelativeRotation` _cameraboom (`self.RotatorCamera`) false false)
  (set `SpringArmComponent.bEnableCameraLag` (`self.Flow`) _cameraboom)
  (set `SpringArmComponent.CameraLagSpeed` (`self.CoefSmooth`) _cameraboom))